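; Raccoon enemy character that roams to random reachable points until pawn sensing spots a pawn, then chases the player to attack.
; Tick re-issues the decision every frame: follow if IsSeeingPlayer, otherwise stop and roam again; the flag effectively never clears once set.
; Attacks randomly play a left or right swipe montage, gated by CanAttack, which FollowPlayer keeps resetting.
; The sphere-trace damage and sound logic is disconnected, so attacks deal no damage here.
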(event OnSeePawn(PawnSensing)
  (params (Pawn :type Pawn%20Object%20Reference))
  ;[1 1 1] Default
  (Variables|Default|SetisSeeingPlayer true))

(event Custom|FollowPlayer
  ;[1 1 1] Follow Player
  (Variables|Default|SetcanAttack true)
  (if (Variables|Default|GetisSeeingPlayer)
    (AI|AIMoveTo self "0, 0, 0" (Game|GetPlayerCharacter 0) 5.0 false
      (:OnSuccess
        (CallFunction|Attack!)))
    (else
      (Variables|Default|SetisSeeingPlayer false))))

(event Custom|Attack!
  ;[1 1 1] Attack!
  (if (Variables|Default|GetcanAttack)
    (Variables|Default|SetcanAttack false)
    (if (> (Math|Random|RandomIntegerinRange 0 1) 0)
      (bind _returnvalue (Animation|PlayAnimMontage "/Game/Medhue_Raccoon/Animation/Raccoon_Attack_L_Montage.Raccoon_Attack_L_Montage" 1.5 "None"))
      (Utilities|FlowControl|Delay _returnvalue)
      (Development|PrintString "Trigger")
      (else
        (bind _returnvalue_2 (Animation|PlayAnimMontage "/Game/Medhue_Raccoon/Animation/Raccoon_Attack_R_Montage.Raccoon_Attack_R_Montage" 1.5 "None"))
        (Utilities|FlowControl|Delay _returnvalue_2)
        (Development|PrintString "HitRight")))
    (Variables|Default|SetcanAttack true)))

(event Custom|AttackOrNot
  ;[1 1 1] Attacking or Not
)

(event Custom|RandomRoaming
  ;[1 1 1] Roaming
  (AI|AIMoveTo self (.RandomLocation (AI|Navigation|GetRandomReachablePointinRadius (Transformation|GetActorLocation) 1e+03 0 0)) 0 5.0 false
    (:OnSuccess
      (CallFunction|Decide))))

(event Custom|Decide
  ;[1 1 1] Decide What To Do
  (if (Variables|Default|GetisSeeingPlayer)
    (CallFunction|FollowPlayer)
    (else
      (CallFunction|RandomRoaming))))

(event EventTick
  (params (DeltaSeconds :type Float%20%28single-precision%29))
  ;[1 1 1] Default
  (if (Variables|Default|GetisSeeingPlayer)
    (CallFunction|FollowPlayer)
    (else
      (Components|Movement|StopMovementImmediately (Variables|Character|GetCharacterMovement))
      (CallFunction|Decide))))

(event EventBeginPlay
  ;[1 1 1] Default
  (CallFunction|Decide))

(fn ConstructionScript)