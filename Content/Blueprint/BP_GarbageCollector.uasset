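; BP_GarbageCollector is a Blueprint with draft logic for an item the first-person player picks up and drops, all currently unreachable.
; The pickup chain checks for a Player tag, caches the character, snap-attaches to its mesh and sets IsBeingHeld.
; A drop chain traces downward from the character and detaches on a hit, without clearing the flag.
; A separate fragment sets the actor transform and clears it.
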(fn ConstructionScript)