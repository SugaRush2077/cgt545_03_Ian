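; Battery pickup actor that recharges the player's battery when touched.
; Its trigger overlap checks for the Player tag, then adds a fixed amount through the first-person character's BPCPlayerStats component.
; It plays a collect sound at its location, destroys itself, then calls DecreaseBattery on the first-person game mode.
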(event OnComponentBeginOverlap(Trigger)
  (params (OverlappedComponent :type Primitive%20Component%20Object%20Reference) (OtherActor :type Actor%20Object%20Reference) (OtherComp :type Primitive%20Component%20Object%20Reference) (OtherBodyIndex :type Integer) (bFromSweep :type Boolean) (SweepResult :type Hit%20Result%20Structure%20%28by%20ref%29))
  (if (Actor|ActorHasTag OtherActor "Player")
    (bind _asbp_first_person_character (Utilities|Casting|CastToBP_FirstPersonCharacter OtherActor))
    (Default|IncreaseBattery (Variables|/Game/FirstPerson/Blueprints/BP_FirstPersonCharacter.BP_FirstPersonCharacter_C|GetBPC_Player_Stats _asbp_first_person_character) 15.0)
    (Audio|PlaySoundatLocation "/Game/MyContent/Sound/collecthealing.collecthealing" (Transformation|GetActorLocation) "0, 0, 0" 1.0 1.0 0.0 0 0 0 0)
    (Actor|DestroyActor)
    (bind _asbp_first_person_game_mode (Utilities|Casting|CastToBP_FirstPersonGameMode (Game|GetGameMode)))
    (Default|DecreaseBattery _asbp_first_person_game_mode)))

(fn ConstructionScript)